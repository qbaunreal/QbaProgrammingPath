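; BP_QbaCharacter is a character Blueprint that puts the default player HUD on screen and keeps its stamina bar current.
; BeginPlay binds a handler to the stamina change delegate, then creates W_DefaultPlayerHUD, seeds it with current and max stamina, and adds it to the viewport.
; Later stamina changes update the bar through that handler if the widget is valid.
; A TODO notes that the HUD setup might move to C++.
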(event `self.ReceiveBeginPlay`
  (add `self.OnStaminaChange` (delegate `OnStaminaChange_Implementation`))
  ;[1 1 1] TODO: might want to move it to c++
  (bind _returnvalue (`|CreateWidget` "/Game/UI/Widgets/W_DefaultPlayerHUD.W_DefaultPlayerHUD_C"))
  (bind _output_get (set `self.BasicHUD` _returnvalue))
  (`/Game/UI/Widgets/W_DefaultPlayerHUD.UpdateStaminaBar` _output_get (`self.GetStamina`) (`self.GetMaxStamina`))
  (`UserWidget.AddToViewport` (`self.BasicHUD`) 0))

(event `OnStaminaChange_Implementation` :!signature `self.OnStaminaChange`
  (params (StaminaValue :type "Float (single-precision)") (MaxStaminaValue :type "Float (single-precision)"))
  (`/Engine/EditorBlueprintResources/StandardMacros.IsValid` (`self.BasicHUD`)
    (:`Is Valid`
      (`/Game/UI/Widgets/W_DefaultPlayerHUD.UpdateStaminaBar` (`self.BasicHUD`) StaminaValue MaxStaminaValue))))

(fn `UserConstructionScript`)